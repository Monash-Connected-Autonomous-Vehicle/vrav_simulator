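; BP_Subaru is a drivable car pawn that passes Enhanced Input actions to its vehicle movement component.
; Steering maps directly, but throttle and brake are crossed: Input_Throttle sets brake input and Input_Break sets throttle input.
; Input_LookAround yaws the spring arm.
; Both spotlights start hidden at construction and BeginPlay, and Input_Light toggles them together on completion, based on the left light's visibility.
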(event Input|EnhancedActionEvents|EnhancedInputActionInput_Throttle
  (params (ActionValue :type Float%20%28double-precision%29) (ElapsedSeconds :type Float%20%28double-precision%29) (TriggeredSeconds :type Float%20%28double-precision%29) (InputAction :type Input%20Action%20Object%20Reference :default "/Game/OurCreatedContent/EnhancedInput/Input_Throttle.Input_Throttle"))
  (:Triggered
    (Class|ChaosVehicleMovementComponent|SetBrakeInput (Variables|Default|GetVehicleMovementComponent) ActionValue :!label _label))
  (:Completed
    (goto _label)))

(event Input|EnhancedActionEvents|EnhancedInputActionInput_Break
  (params (ActionValue :type Float%20%28double-precision%29) (ElapsedSeconds :type Float%20%28double-precision%29) (TriggeredSeconds :type Float%20%28double-precision%29) (InputAction :type Input%20Action%20Object%20Reference :default "/Game/OurCreatedContent/EnhancedInput/Input_Break.Input_Break"))
  (:Triggered
    (Class|ChaosVehicleMovementComponent|SetThrottleInput (Variables|Default|GetVehicleMovementComponent) ActionValue :!label _label))
  (:Completed
    (goto _label)))

(event Input|EnhancedActionEvents|EnhancedInputActionInput_Steering
  (params (ActionValue :type Float%20%28double-precision%29) (ElapsedSeconds :type Float%20%28double-precision%29) (TriggeredSeconds :type Float%20%28double-precision%29) (InputAction :type Input%20Action%20Object%20Reference :default "/Game/OurCreatedContent/EnhancedInput/Input_Steering.Input_Steering"))
  (:Triggered
    (Class|ChaosVehicleMovementComponent|SetSteeringInput (Variables|Default|GetVehicleMovementComponent) ActionValue :!label _label))
  (:Completed
    (goto _label)))

(event Input|EnhancedActionEvents|EnhancedInputActionInput_LookAround
  (params (ActionValue :type Float%20%28double-precision%29) (ElapsedSeconds :type Float%20%28double-precision%29) (TriggeredSeconds :type Float%20%28double-precision%29) (InputAction :type Input%20Action%20Object%20Reference :default "/Game/OurCreatedContent/EnhancedInput/Input_LookAround.Input_LookAround"))
  (:Triggered
    (Transformation|AddLocalRotation (Variables|Default|GetSpringArm) (Math|Rotator|MakeRotator 0.0 0.0 ActionValue) false false)))

(event Input|EnhancedActionEvents|EnhancedInputActionInput_Light
  (params (ActionValue :type Boolean) (ElapsedSeconds :type Float%20%28double-precision%29) (TriggeredSeconds :type Float%20%28double-precision%29) (InputAction :type Input%20Action%20Object%20Reference :default "/Game/OurCreatedContent/EnhancedInput/Input_Light.Input_Light"))
  (:Completed
    (Rendering|SetVisibility (Variables|Default|GetSpotLight_R) (not (Rendering|IsVisible (Variables|Default|GetSpotLight_L))) false)))

(event EventBeginPlay
  (Rendering|SetVisibility (Variables|Default|GetSpotLight_R) false false))

(fn ConstructionScript
  (Rendering|SetVisibility (Variables|Default|GetSpotLight_R) false false))