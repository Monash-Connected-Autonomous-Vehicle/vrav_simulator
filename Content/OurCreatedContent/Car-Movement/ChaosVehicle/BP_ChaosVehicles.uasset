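; BP_ChaosVehicles is an AI-steered Chaos vehicle that follows the facing direction of an AI_SphereOLD child actor.
; Each tick it applies half throttle, compares desired and current yaw, and costs left versus right turns across the wraparound.
; Outside the yaw tolerance it steers fully toward the cheaper side, braking if above minimum speed; nothing resets either input.
; StopCarMovement brakes and flags goal contact, but Tick never checks that flag.
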(event EventBeginPlay
  (bind _asai_sphere_old (Utilities|Casting|CastToAI_SphereOLD (Variables|/Script/Engine.ChildActorComponent|GetChildActor (Variables|Default|GetNavComponent))))
  (Variables|Default|SetCarAISphere _asai_sphere_old)
  (Variables|Default|SetHasTouchedGoal false))

(event EventTick
  (params (DeltaSeconds :type Float%20%28single-precision%29))
  (bind _vehiclemovementcomponent (Variables|Default|GetVehicleMovementComponent))
  (Class|ChaosVehicleMovementComponent|SetThrottleInput (Variables|Default|GetVehicleMovementComponent) 0.5)
  (CallFunction|SetDesiredYawVar)
  (CallFunction|SetCurrentYawVar)
  (CallFunction|CalculateCostOfSteering)
  (Development|PrintString (Utilities|String|Append "Desired Yaw: " (Utilities|String|ToString(Float) (Variables|Default|GetDesiredYaw)) " 
Current Yaw: " (Utilities|String|ToString(Float) (Variables|Default|GetCurrentYaw)) " 
Speed:  " (Utilities|String|ToString(Float) (Vehicle|GetForwardSpeed (Variables|Default|GetVehicleMovementComponent)))) true true "(R=0.000000,G=0.660000,B=1.000000,A=1.000000)" (Utilities|Time|GetWorldDeltaSeconds))
  (bind _returnvalue (CallFunction|IsWithinAcceptableYawRange))
  (if (not _returnvalue)
    (bind _returnvalue_2 (CallFunction|IsMovingAboveMinimumSPeed))
    (if (and _returnvalue_2 (not _returnvalue))
      (Class|ChaosVehicleMovementComponent|SetBrakeInput (Variables|Default|GetVehicleMovementComponent) 1.0))
    (if (> (Variables|Default|GetSteerRightCost) (Variables|Default|GetSteerLeftCost))
      (Class|ChaosVehicleMovementComponent|SetSteeringInput _vehiclemovementcomponent -1.0)
      (else
        (Class|ChaosVehicleMovementComponent|SetSteeringInput _vehiclemovementcomponent 1.0)))))

(fn ConstructionScript)

(fn SetDesiredYawVar
  (Variables|Default|SetDesiredYaw (+ 1.8e+02 (.Yaw (Math|Vector|GetYawPitchfromVector (Math|Vector|GetForwardVector (Variables|/Game/OurCreatedContent/Car-Movement/ChaosVehicle/AI_SphereOLD.AI_SphereOLD_C|GetFacingDirectionVar (Variables|Default|GetCarAISphere))))))))

(fn SetCurrentYawVar
  (Variables|Default|SetCurrentYaw (+ 1.8e+02 (.Yaw (Math|Vector|GetYawPitchfromVector (Math|Vector|GetForwardVector (Variables|Character|GetMesh)))))))

(fn StopCarMovement
  (bind _vehiclemovementcomponent (Variables|Default|GetVehicleMovementComponent))
  (Class|ChaosVehicleMovementComponent|SetThrottleInput _vehiclemovementcomponent 0.0)
  (Class|ChaosVehicleMovementComponent|SetBrakeInput _vehiclemovementcomponent 1.0)
  (Class|ChaosVehicleMovementComponent|SetHandbrakeInput _vehiclemovementcomponent true)
  (Variables|Default|SetHasTouchedGoal true))

(fn CalculateCostOfSteering
  (if (> (Variables|Default|GetDesiredYaw) (Variables|Default|GetCurrentYaw))
    (Variables|Default|SetSteerRightCost (- (Variables|Default|GetDesiredYaw) (Variables|Default|GetCurrentYaw)))
    (Variables|Default|SetSteerLeftCost (+ (Variables|Default|GetCurrentYaw) (- 3.6e+02 (Variables|Default|GetDesiredYaw))))
    (else
      (Variables|Default|SetSteerRightCost (+ (Variables|Default|GetDesiredYaw) (- 3.6e+02 (Variables|Default|GetCurrentYaw))))
      (Variables|Default|SetSteerLeftCost (- (Variables|Default|GetCurrentYaw) (Variables|Default|GetDesiredYaw))))))

(fn IsWithinAcceptableYawRange
  (return (or (< (Variables|Default|GetSteerLeftCost) (Variables|Default|GetAcceptableYawRange)) (< (Variables|Default|GetSteerRightCost) (Variables|Default|GetAcceptableYawRange)))))

(fn IsMovingAboveMinimumSPeed
  (return (> (Vehicle|GetForwardSpeed (Variables|Default|GetVehicleMovementComponent)) (Variables|Default|GetMinimumSpeed))))