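; SubaruVehicle is a drivable Chaos wheeled vehicle pawn for the Subaru car.
; Enhanced Input actions for throttle, steering and brake pass their values straight to the vehicle movement component.
; On BeginPlay it casts that component to ChaosWheeledVehicleMovementComponent and stores it in a VehicleMovement variable, which the input handlers do not use.
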(event Input|EnhancedActionEvents|EnhancedInputActionInput_Throttle
  (params (ActionValue :type Float%20%28double-precision%29) (ElapsedSeconds :type Float%20%28double-precision%29) (TriggeredSeconds :type Float%20%28double-precision%29) (InputAction :type Input%20Action%20Object%20Reference :default "/Game/car-hyperrealism/EnhancedInput/Input_Throttle.Input_Throttle"))
  ;[1 1 1] Movement
  (:Triggered
    (Class|ChaosVehicleMovementComponent|SetThrottleInput (Variables|Default|GetVehicleMovementComponent) ActionValue)))

(event Input|EnhancedActionEvents|EnhancedInputActionInput_Break
  (params (ActionValue :type Float%20%28double-precision%29) (ElapsedSeconds :type Float%20%28double-precision%29) (TriggeredSeconds :type Float%20%28double-precision%29) (InputAction :type Input%20Action%20Object%20Reference :default "/Game/car-hyperrealism/EnhancedInput/Input_Break.Input_Break"))
  ;[1 1 1] Movement
  (:Triggered
    (Class|ChaosVehicleMovementComponent|SetBrakeInput (Variables|Default|GetVehicleMovementComponent) ActionValue)))

(event Input|EnhancedActionEvents|EnhancedInputActionInput_Steering
  (params (ActionValue :type Float%20%28double-precision%29) (ElapsedSeconds :type Float%20%28double-precision%29) (TriggeredSeconds :type Float%20%28double-precision%29) (InputAction :type Input%20Action%20Object%20Reference :default "/Game/car-hyperrealism/EnhancedInput/Input_Steering.Input_Steering"))
  ;[1 1 1] Movement
  (:Triggered
    (Class|ChaosVehicleMovementComponent|SetSteeringInput (Variables|Default|GetVehicleMovementComponent) ActionValue)))

(event EventBeginPlay
  ;[1 1 1] Setting Movement Component
  (bind _aschaos_wheeled_vehicle_movement_component (Utilities|Casting|CastToChaosWheeledVehicleMovementComponent (Variables|Default|GetVehicleMovementComponent)))
  (Variables|Default|SetVehicleMovement _aschaos_wheeled_vehicle_movement_component))

(fn ConstructionScript)