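; Sky sphere actor that drives the sky dome material and an optional day-night cycle for an assigned directional light.
; Construction script builds a dynamic material for sun, clouds and stars, taking colors from sun-height curves or manual values, and can recapture the sky light.
; A timeline pitches the light, refreshes the material each update, switches off light and shadows when the sun is low, and can tint the light from the horizon curve.
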(event Custom|Update%20SKyLight
  (bind _skylight (Variables|Default|GetSkyLight))
  (Utilities|IsValid _skylight
    (:Is%20Valid
      (Class|SkyLightComponent|RecaptureSky (Variables|/Script/Engine.SkyLight|GetLightComponent _skylight)))))

(event EventBeginPlay
  (bind _sun_height (Variables|Overridesettings|GetSun%20height))
  (bind _directional_light_actor (Variables|Default|GetDirectional%20light%20actor))
  (bind _directional_light_actor_2 (Variables|Default|GetDirectional%20light%20actor))
  (bind _returnvalue (Transformation|GetActorRotation _directional_light_actor))
  (bind _lightcomponent (Variables|/Script/Engine.Light|GetLightComponent _directional_light_actor_2))
  (bind (_roll _pitch _yaw) (Math|Rotator|BreakRotator _returnvalue))
  (Utilities|IsValid (Variables|Default|GetDirectional%20light%20actor)
    (:Is%20Valid
      ;[1 1 1] Day Night Cycle
      (Utilities|FlowControl|Sequence
        (:then_0
          (Utilities|FlowControl|DoOnce false
            (:Completed
              (Variables|Default|SetCurrentLightIntensity (Variables|/Script/Engine.LightComponentBase|GetIntensity (Variables|/Script/Engine.Light|GetLightComponent (Variables|Default|GetDirectional%20light%20actor)))))))
        (:then_1
          (if (Variables|EScenelighting|GetActivateDayNightCycle?)
            (bind _sun_position (Timeline|DayNightCycle Play)
              (:Update
                (bind _output_get (Variables|EScenelighting|SetSun%20position%20Y%20output (+ (* (Variables|EScenelighting|GetSpeed%20update%20factor) _sun_position) (Variables|EScenelighting|GetSun%20position%20%28Y%29))))
                (Transformation|SetActorRotation (Variables|Default|GetDirectional%20light%20actor) (Math|Rotator|MakeRotator (Variables|EScenelighting|GetSun%20Roll%20%28X%29) _output_get (Variables|EScenelighting|GetSun%20Yaw%20%28Z%29)))
                (CallFunction|UpdateSunDirection)
                (if (not (and (<= 0.022222 _sun_height) (>= _sun_height -0.011111)))
                  (Rendering|Components|Light|SetCastShadows _lightcomponent false)
                  (Rendering|Components|Light|SetIntensity _lightcomponent 0.0)
                  (else
                    (Rendering|Components|Light|SetCastShadows _lightcomponent true)
                    (Rendering|Components|Light|SetIntensity _lightcomponent (Variables|Default|GetCurrentLightIntensity))))
                (if (Variables|EScenelighting|GetUseAutomaticLightColor)
                  (Rendering|Components|Light|SetLightColor (Variables|/Script/Engine.Light|GetLightComponent (Variables|Default|GetDirectional%20light%20actor)) (Math|Curves|GetLinearColorValue (Variables|Default|GetHorizon%20color%20curve) (Variables|Overridesettings|GetSun%20height)) true)))
              (:Finished
                (Transformation|SetActorRotation _directional_light_actor (Math|Rotator|MakeRotator _roll _pitch (+ _yaw (Variables|EScenelighting|GetSun%20Yaw%20%28Z%29%20Cycle%20rot))))
                (Variables|EScenelighting|SetSun%20position%20Y%20output 0.0)))))))))

(fn ConstructionScript
  (bind _directional_light_actor (Variables|Default|GetDirectional%20light%20actor))
  (bind _skylight (Variables|Default|GetSkyLight))
  (Utilities|IsValid _skylight
    (:Is%20Valid
      (if (Variables|EScenelighting|GetAuto%20Update%20Sky%20Light)
        (Class|SkyLightComponent|RecaptureSky (Variables|/Script/Engine.SkyLight|GetLightComponent _skylight))))
    (:Is%20Not%20Valid
      _))
  (bind _returnvalue (Rendering|Material|CreateDynamicMaterialInstance (Variables|BP_Skydome|GetSky%20Sphere%20mesh) 0 "/Engine/EngineSky/M_Sky_Panning_Clouds2.M_Sky_Panning_Clouds2" "None" :!class /Script/Engine.PrimitiveComponent))
  (Variables|Default|SetSky%20material _returnvalue)
  (Utilities|FlowControl|Sequence
    (:then_0
      _)
    (:then_1
      (Utilities|IsValid _directional_light_actor
        (:Is%20Valid
          (Transformation|SetActorRotation _directional_light_actor (Math|Rotator|MakeRotator (Variables|EScenelighting|GetSun%20Roll%20%28X%29) (Variables|EScenelighting|GetSun%20position%20%28Y%29) (Variables|EScenelighting|GetSun%20Yaw%20%28Z%29)))))))
  (if (Variables|EScenelighting|GetRefresh%20material) ; Updating bool in details panel causes construction script to run again
    _
    (else
      _))
  (Variables|EScenelighting|SetRefresh%20material false)
  (Rendering|Material|SetScalarParameterValue (Variables|Default|GetSky%20material) "Sun Radius" (Variables|EScenelighting|GetSun%20Radius) :!class /Script/Engine.MaterialInstanceDynamic)
  (Utilities|IsValid (Variables|Default|GetDirectional%20light%20actor) ; Has a directional light been assigned?
    (:Is%20Valid
      (Rendering|Components|Light|SetLightColor (Variables|/Script/Engine.Light|GetLightComponent (Variables|Default|GetDirectional%20light%20actor)) (Variables|EScenelighting|GetSun%20Color) true)
      (Rendering|Material|SetVectorParameterValue (Variables|Default|GetSky%20material) "Light direction" (Math|Conversions|ToLinearColor(Vector) (Math|Rotator|GetRotationXVector (Transformation|GetActorRotation (Variables|Default|GetDirectional%20light%20actor)))) :!class /Script/Engine.MaterialInstanceDynamic)
      (Rendering|Material|SetVectorParameterValue (Variables|Default|GetSky%20material) "Sun color" (Math|Conversions|ToLinearColor(Color) (Variables|/Script/Engine.LightComponentBase|GetLightColor (Variables|/Script/Engine.Light|GetLightComponent (Variables|Default|GetDirectional%20light%20actor)))) :!class /Script/Engine.MaterialInstanceDynamic)
      (Variables|Overridesettings|SetSun%20height (Math|Float|MapRangeUnclamped (.Pitch (Math|Rotator|BreakRotator (Transformation|GetActorRotation (Variables|Default|GetDirectional%20light%20actor)))) 0.0 -9e+01 0.0 1.0)))
    (:Is%20Not%20Valid
      (Rendering|Material|SetVectorParameterValue (Variables|Default|GetSky%20material) "Light direction" (Math|Conversions|ToLinearColor(Vector) (Math|Rotator|GetRotationXVector (Math|Rotator|MakeRotator 0.0 (Math|Float|MapRangeUnclamped (Variables|Overridesettings|GetSun%20height) -1.0 1.0 9e+01 -9e+01) (.Yaw (Math|Rotator|BreakRotator (Transformation|GetActorRotation)))))) :!class /Script/Engine.MaterialInstanceDynamic)
      (Rendering|Material|SetVectorParameterValue (Variables|Default|GetSky%20material) "Sun color" (Math|Color|Lerp(LinearColor) "(R=1.000000,G=0.221000,B=0.040000,A=1.000000)" "(R=0.954000,G=0.901000,B=0.744120,A=1.000000)" (Math|Float|Clamp(Float) (+ (Variables|Overridesettings|GetSun%20height) 0.2))) :!class /Script/Engine.MaterialInstanceDynamic)))
  (if (Variables|EScenelighting|GetColors%20determined%20by%20sun%20position)
    (Rendering|Material|SetVectorParameterValue (Variables|Default|GetSky%20material) "Horizon color" (Math|Curves|GetLinearColorValue (Variables|Default|GetHorizon%20color%20curve) (Variables|Overridesettings|GetSun%20height)) :!class /Script/Engine.MaterialInstanceDynamic)
    (Rendering|Material|SetVectorParameterValue (Variables|Default|GetSky%20material) "Zenith color" (Math|Curves|GetLinearColorValue (Variables|Default|GetZenith%20color%20curve) (Variables|Overridesettings|GetSun%20height)) :!class /Script/Engine.MaterialInstanceDynamic)
    (Rendering|Material|SetVectorParameterValue (Variables|Default|GetSky%20material) "Cloud color" (Math|Curves|GetLinearColorValue (Variables|Default|GetCloud%20color%20curve) (Variables|Overridesettings|GetSun%20height)) :!class /Script/Engine.MaterialInstanceDynamic)
    (Rendering|Material|SetScalarParameterValue (Variables|Default|GetSky%20material) "Horizon falloff" (Math|Float|Lerp 3.0 7.0 (Math|Float|Absolute(Float) (Variables|Overridesettings|GetSun%20height))) :!class /Script/Engine.MaterialInstanceDynamic)
    (else
      (Rendering|Material|SetVectorParameterValue (Variables|Default|GetSky%20material) "Horizon color" (Variables|Overridesettings|GetHorizon%20color) :!class /Script/Engine.MaterialInstanceDynamic)
      (Rendering|Material|SetVectorParameterValue (Variables|Default|GetSky%20material) "Zenith color" (Variables|Overridesettings|GetZenith%20Color) :!class /Script/Engine.MaterialInstanceDynamic)
      (Rendering|Material|SetVectorParameterValue (Variables|Default|GetSky%20material) "Overall color" (Variables|Overridesettings|GetOverall%20Color) :!class /Script/Engine.MaterialInstanceDynamic)
      (Rendering|Material|SetVectorParameterValue (Variables|Default|GetSky%20material) "Cloud color" (Variables|Overridesettings|GetCloud%20color) :!class /Script/Engine.MaterialInstanceDynamic)
      (Rendering|Material|SetScalarParameterValue (Variables|Default|GetSky%20material) "Horizon falloff" (Variables|Overridesettings|GetHorizon%20Falloff) :!class /Script/Engine.MaterialInstanceDynamic)))
  (Rendering|Material|SetScalarParameterValue (Variables|Default|GetSky%20material) "Cloud speed" (Variables|EScenelighting|GetCloud%20speed) :!class /Script/Engine.MaterialInstanceDynamic)
  (Rendering|Material|SetScalarParameterValue (Variables|Default|GetSky%20material) "Sun brightness" (Variables|EScenelighting|GetSun%20brightness) :!class /Script/Engine.MaterialInstanceDynamic)
  (Rendering|Material|SetScalarParameterValue (Variables|Default|GetSky%20material) "Sun height" (Math|Float|SelectFloat (Math|Float|Absolute(Float) (Variables|Overridesettings|GetSun%20height)) 0.0 (< (Variables|Overridesettings|GetSun%20height) 0.0)) :!class /Script/Engine.MaterialInstanceDynamic)
  (Rendering|Material|SetScalarParameterValue (Variables|Default|GetSky%20material) "Cloud opacity" (Variables|EScenelighting|GetCloud%20opacity) :!class /Script/Engine.MaterialInstanceDynamic)
  (Rendering|Material|SetScalarParameterValue (Variables|Default|GetSky%20material) "Stars brightness" (Variables|EScenelighting|GetStars%20brightness) :!class /Script/Engine.MaterialInstanceDynamic))

(fn UpdateSunDirection
  (bind _directional_light_actor (Variables|Default|GetDirectional%20light%20actor))
  (bind _sky_material (Variables|Default|GetSky%20material))
  (bind _sky_material_2 (Variables|Default|GetSky%20material))
  (Utilities|IsValid _directional_light_actor
    (:Is%20Valid
      (Rendering|Material|SetVectorParameterValue _sky_material "Light direction" (Math|Conversions|ToLinearColor(Vector) (Math|Rotator|GetRotationXVector (Transformation|GetActorRotation _directional_light_actor))) :!class /Script/Engine.MaterialInstanceDynamic)
      (Rendering|Material|SetVectorParameterValue _sky_material "Sun color" (Math|Conversions|ToLinearColor(Color) (Variables|/Script/Engine.LightComponentBase|GetLightColor (Variables|/Script/Engine.Light|GetLightComponent (Variables|Default|GetDirectional%20light%20actor)))) :!class /Script/Engine.MaterialInstanceDynamic)
      (Variables|Overridesettings|SetSun%20height (Math|Float|MapRangeUnclamped (.Pitch (Math|Rotator|BreakRotator (Transformation|GetActorRotation (Variables|Default|GetDirectional%20light%20actor)))) 0.0 -9e+01 0.0 1.0))
      (Rendering|Material|SetVectorParameterValue _sky_material_2 "Horizon color" (Math|Curves|GetLinearColorValue (Variables|Default|GetHorizon%20color%20curve) (Variables|Overridesettings|GetSun%20height)) :!class /Script/Engine.MaterialInstanceDynamic)
      (Rendering|Material|SetVectorParameterValue _sky_material_2 "Zenith color" (Math|Curves|GetLinearColorValue (Variables|Default|GetZenith%20color%20curve) (Variables|Overridesettings|GetSun%20height)) :!class /Script/Engine.MaterialInstanceDynamic)
      (Rendering|Material|SetVectorParameterValue _sky_material_2 "Cloud color" (Math|Curves|GetLinearColorValue (Variables|Default|GetCloud%20color%20curve) (Variables|Overridesettings|GetSun%20height)) :!class /Script/Engine.MaterialInstanceDynamic)
      (Rendering|Material|SetScalarParameterValue _sky_material_2 "Horizon falloff" (Math|Float|Lerp 3.0 8.0 (Math|Float|Absolute(Float) (Variables|Overridesettings|GetSun%20height))) :!class /Script/Engine.MaterialInstanceDynamic)
      (Rendering|Material|SetScalarParameterValue _sky_material_2 "Sun height" (Math|Float|SelectFloat (Math|Float|Absolute(Float) (Variables|Overridesettings|GetSun%20height)) 0.0 (< (Variables|Overridesettings|GetSun%20height) 0.0)) :!class /Script/Engine.MaterialInstanceDynamic))))